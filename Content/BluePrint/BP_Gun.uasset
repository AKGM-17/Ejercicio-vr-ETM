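; BP_Gun is a gun Blueprint that fires bullets and tracks its ammunition.
; Disparar spawns a Bala at the Arrow component's world transform while Ammo remains, then decrements it and prints the rounds left out of six in Spanish.
; With no ammo it prints an empty warning instead, and Recargar instantly resets Ammo to a full six.
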(event `Disparar`
  (if (> (`self.Ammo`) 0)
    (`|SpawnActorFromClass` "/Game/BluePrint/Bala.Bala_C" (`SceneComponent.K2_GetComponentToWorld` (`self.Arrow`)) "Undefined" "MultiplyWithRoot" null null)
    (`/Engine/EditorBlueprintResources/StandardMacros.DecrementInt` (`self.Ammo`)
      (:`  `
        (`KismetSystemLibrary.PrintString` (`KismetTextLibrary.Conv_TextToString` (`|FormatText` "Te quedan {Municion}/6 balas." (`self.Ammo`))))))
    (else
      (`KismetSystemLibrary.PrintString` "Sin munición."))))

(event `Recargar`
  (set `self.Ammo` 6))

(fn `UserConstructionScript`)