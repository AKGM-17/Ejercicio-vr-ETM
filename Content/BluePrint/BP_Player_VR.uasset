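; VR player Blueprint that picks up a gun and routes fire and reload input to it.
; On BeginPlay it adds the IMC_Pistola Enhanced Input mapping context.
; The first overlap of StaticMesh1 with a BP_Gun destroys that gun, spawns a replacement snapped to Left, hides StaticMesh1 and sets Armado.
; The Disparar (fire) and Recargar (reload) actions call the held gun only while Armado is true.
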(event `self.ReceiveBeginPlay`
  (`EnhancedInputSubsystemInterface.AddMappingContext` (pcsubsystem `EnhancedInputLocalPlayerSubsystem` (`GameplayStatics.GetPlayerController` 0)) "/Game/Input/IMC_Pistola.IMC_Pistola" 0 (struct)))

(event `self.StaticMesh1.OnComponentBeginOverlap`
  (params (OverlappedComponent :type "PrimitiveComponent Object Reference") (OtherActor :type "Actor Object Reference") (OtherComp :type "PrimitiveComponent Object Reference") (OtherBodyIndex :type Integer) (bFromSweep :type Boolean) (SweepResult :type "HitResult Structure (by ref)"))
  (bind _asbp_gun (cast `/Game/BluePrint/BP_Gun` OtherActor))
  (`/Engine/EditorBlueprintResources/StandardMacros.DoOnce` false
    (:`Completed`
      (`self.K2_DestroyActor` _asbp_gun)
      (`SceneComponent.SetHiddenInGame` (`self.StaticMesh1`) false false)
      (bind _returnvalue (`|SpawnActorFromClass` "/Game/BluePrint/BP_Gun.BP_Gun_C" (`SceneComponent.K2_GetComponentToWorld` (`self.Left`)) "Undefined" "MultiplyWithRoot" null null))
      (bind _output_get (set `self.Gun` _returnvalue))
      (`self.K2_AttachToComponent` _output_get (`self.Left`) "None" "SnapToTarget" "SnapToTarget" "SnapToTarget" true)
      (`SceneComponent.SetVisibility` (`self.StaticMesh1`) false false)
      (set `self.Armado` true))))

(event `EnhancedInput|/Game/Input/Disparar`
  (params (ActionValue :type Boolean) (ElapsedSeconds :type "Float (double-precision)") (TriggeredSeconds :type "Float (double-precision)") (InputAction :type "InputAction Object Reference" :default "/Game/Input/Disparar.Disparar"))
  (:`Started`
    (if (`self.Armado`)
      (`/Game/BluePrint/BP_Gun.Disparar` (`self.Gun`)))))

(event `EnhancedInput|/Game/Input/Recargar`
  (params (ActionValue :type Boolean) (ElapsedSeconds :type "Float (double-precision)") (TriggeredSeconds :type "Float (double-precision)") (InputAction :type "InputAction Object Reference" :default "/Game/Input/Recargar.Recargar"))
  (:`Triggered`
    (if (`self.Armado`)
      (`/Game/BluePrint/BP_Gun.Recargar` (`self.Gun`)))))

(fn `UserConstructionScript`)